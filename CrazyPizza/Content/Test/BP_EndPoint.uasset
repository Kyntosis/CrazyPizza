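; BP_EndPoint is a finish-point trigger for a vehicle game that awards a win and bonus time.
; On BeginPlay it caches the HUD and countdown widget from the vehicle player controller, using short delays.
; When a vehicle pawn overlaps its box and the countdown is at least the win threshold, it briefly shows YouWin, adds bonus time to the countdown and then destroys itself.
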(event `self.ReceiveBeginPlay`
  (bind _asbp_vehicle_adv_player_controller (cast `/Game/VehicleTemplate/Blueprints/BP_VehicleAdvPlayerController` (`GameplayStatics.GetPlayerController` 0)))
  (bind _output_get (set `self.As BP Vehicle Adv Player Controller` _asbp_vehicle_adv_player_controller))
  (`KismetSystemLibrary.Delay` 0.2)
  (bind _vehiclehud (`/Game/VehicleTemplate/Blueprints/BP_VehicleAdvPlayerController.VehicleHud` _output_get))
  (set `self.Vehicle Hud` _vehiclehud)
  (`KismetSystemLibrary.Delay` 0.2)
  (set `self.BPW Countdown` (`/Game/VehicleTemplate/UI/UI_Vehicle.BPW_Countdown` _vehiclehud)))

(event `self.Boxcollision.OnComponentBeginOverlap`
  (params (OverlappedComponent :type "PrimitiveComponent Object Reference") (OtherActor :type "Actor Object Reference") (OtherComp :type "PrimitiveComponent Object Reference") (OtherBodyIndex :type Integer) (bFromSweep :type Boolean) (SweepResult :type "HitResult Structure (by ref)"))
  (bind _bpw_countdown (`self.BPW Countdown`))
  (cast `/Game/VehicleTemplate/Blueprints/BP_VehicleAdvPawnBase` OtherActor)
  (`KismetSystemLibrary.PrintString` "colliding")
  (if (>= (`/Game/UI/BPW_Countdown.Countdown` (`self.BPW Countdown`)) (`self.WinConditionTimer`))
    (`KismetSystemLibrary.PrintString` "Yeahh")
    (bind _vehicle_hud (`self.Vehicle Hud`)
      (:`then`
        (bind _youwin (`/Game/VehicleTemplate/UI/UI_Vehicle.YouWin` _vehicle_hud))
        (`Widget.SetVisibility` _youwin "Visible")
        (set `/Game/UI/BPW_Countdown.Countdown` (+ (`/Game/UI/BPW_Countdown.Countdown` _bpw_countdown) (`self.BonusTime`)) _bpw_countdown)
        (`KismetSystemLibrary.Delay` 2.0)
        (`Widget.SetVisibility` _youwin "Hidden")
        (`self.K2_DestroyActor`))
      (:`else`))))

(fn `UserConstructionScript`)